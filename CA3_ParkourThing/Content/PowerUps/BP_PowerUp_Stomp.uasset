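; BP_PowerUp_Stomp is a pickup that grants the player character the Stomp power-up on overlap.
; If the first character found lacks Stomper, it sets that flag on player 0's character and shows the Stomp element in the W_PowerUps widget.
; The mesh, which has collision disabled, hides for a few seconds after a grant, then reappears.
; A DoOnce gates overlaps, and its delayed reset sits on a parallel Sequence branch.
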(event `self.ReceiveBeginPlay`
  (`PrimitiveComponent.SetCollisionEnabled` (`self.StaticMeshComponent`) "NoCollision"))

(event `self.ReceiveActorBeginOverlap`
  (params (OtherActor :type "Actor Object Reference"))
  (bind _staticmeshcomponent (`self.StaticMeshComponent`))
  (`/Engine/EditorBlueprintResources/StandardMacros.DoOnce` false :!label _label
    (:`Completed`
      (`|ExecutionSequence`
        (:`then_0`
          (bind _outactors (`GameplayStatics.GetAllActorsOfClass` "/Game/ThirdPerson/Blueprints/BP_ThirdPersonCharacter.BP_ThirdPersonCharacter_C"))
          (if (not (`/Game/ThirdPerson/Blueprints/BP_ThirdPersonCharacter.Stomper` (`|GetArrayItem` _outactors)))
            (bind _asbp_third_person_character (cast `/Game/ThirdPerson/Blueprints/BP_ThirdPersonCharacter` (`GameplayStatics.GetPlayerCharacter` 0)))
            (set `/Game/ThirdPerson/Blueprints/BP_ThirdPersonCharacter.Stomper` true _asbp_third_person_character)
            (bind _foundwidgets (`WidgetBlueprintLibrary.GetAllWidgetsOfClass` "/Game/UI/W_PowerUps.W_PowerUps_C"))
            (`Widget.SetRenderOpacity` (`/Game/UI/W_PowerUps.SB_Stomp` (`|GetArrayItem` _foundwidgets)) 1.0)
            (`SceneComponent.SetVisibility` _staticmeshcomponent false false)
            (`KismetSystemLibrary.Delay` 5.0)
            (`SceneComponent.SetVisibility` _staticmeshcomponent true false)))
        (:`then_1`
          (`KismetSystemLibrary.Delay` 5.0)
          (goto _label :!via `Reset`))))))

(fn `UserConstructionScript`)